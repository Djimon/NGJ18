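; Level database actor that holds a shared, length-capped supply queue of resource demands from bases.
; AddDemand appends base and resource numbers packed into a Vector2D, or prints a message and returns false when full.
; GetNextSupply pops the oldest entry, making the queue first-in, first-out.
; BeginPlay clears the queue and gathers all Base_BP actors, but the loop that would store their positions is unconnected.
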(event `self.ReceiveBeginPlay`
  (`KismetArrayLibrary.Array_Clear` (`self.SupplyChain`))
  (bind _outactors (`GameplayStatics.GetAllActorsOfClass` "/Game/Blueprints/Base_BP.Base_BP_C")))

(fn `AddDemand`
  (params (`Base No` :type Integer) (`Ress No` :type Integer))
  (returns (DemandSucceded :type Boolean))
  (if (>= (`KismetArrayLibrary.Array_Length` (`self.SupplyChain`)) (`self.MaxSupplyChainLength`))
    (set `self.ReturnDemand` false)
    (`KismetSystemLibrary.PrintString` "SupplyChain is Full")
    (else
      (set `self.ReturnDemand` true)
      (`KismetArrayLibrary.Array_Add` (`self.SupplyChain`) (`KismetMathLibrary.MakeVector2D` (`KismetMathLibrary.Conv_IntToDouble` `Base No`) (`KismetMathLibrary.Conv_IntToDouble` `Ress No`)))))
  (return (`self.ReturnDemand`)))

(fn `GetNextSupply`
  (returns (NextSupply :type "Vector2D Structure"))
  (bind _supplychain (`self.SupplyChain`))
  ;[1 1 1] Check if Array is empty
  (if (!= (`KismetArrayLibrary.Array_Length` _supplychain) 0)
    (set `self.NextSupply` (`|GetArrayItem` _supplychain))
    (`KismetArrayLibrary.Array_Remove` _supplychain)
    (return (`self.NextSupply`))))

(fn `UserConstructionScript`)