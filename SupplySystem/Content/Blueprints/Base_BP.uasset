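; Base actor for a resource supply system, holding Water, Food and Tools stocks and a base number derived from the Base_BP actor count.
; A looping timer paced by production speed increments the produced resource, set to Water on BeginPlay.
; A second timer detects low stocks and calls OrderRessources, which registers demand with LevelDatabseActor.
; Its SupplyChain duplicate check uses a (Demand, base number) vector before Demand updates to the requested resource.
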(event `self.ReceiveBeginPlay`
  (bind _outactors (`GameplayStatics.GetAllActorsOfClass` "Base_BP_C"))
  (bind _result (`/Engine/EditorBlueprintResources/StandardMacros.IncrementInt` (`KismetArrayLibrary.Array_Length` _outactors))
    (:`  `
      (set `self.iBaseNo` _result)
      (set `self.ERess` "NewEnumerator0")
      (set `self.Water` 10)
      (set `self.Food` 10)
      (set `self.Tools` 10)
      (`KismetSystemLibrary.K2_SetTimerDelegate` (delegate `Base_Gathering`) (/ (`self.MaxProductionTime`) (`self.ProductionSpeed`)) true)
      (`KismetSystemLibrary.K2_SetTimerDelegate` (delegate `DemandSupply`) 10.0 true))))

(event `Base_Gathering`
  (switch `/Game/Blueprints/ERessorces` (`self.ERess`)
    (:`NewEnumerator0`
      (`/Engine/EditorBlueprintResources/StandardMacros.IncrementInt` (`self.Water`)))
    (:`NewEnumerator1`
      (`/Engine/EditorBlueprintResources/StandardMacros.IncrementInt` (`self.Food`)))
    (:`NewEnumerator2`
      (`/Engine/EditorBlueprintResources/StandardMacros.IncrementInt` (`self.Tools`)))))

(event `DemandSupply`
  (if (<= (`self.Water`) 1)
    (`self.OrderRessources` "NewEnumerator0"))
  (if (<= (`self.Food`) 1)
    (`self.OrderRessources` "NewEnumerator1"))
  (if (<= (`self.Tools`) 1)
    (`self.OrderRessources` "NewEnumerator2")))

(fn `OrderRessources`
  (params (Ressoruce :type "/Game/Blueprints/ERessorces Enum" :default "NewEnumerator0"))
  (bind _outactors (`GameplayStatics.GetAllActorsOfClass` "/Game/Blueprints/LevelDatabseActor.LevelDatabseActor_C"))
  (for _array_element _outactors
    _)
  (if (not (!= (`KismetArrayLibrary.Array_Find` (`/Game/Blueprints/LevelDatabseActor.SupplyChain` _array_element) (`KismetMathLibrary.MakeVector2D` (`KismetMathLibrary.Conv_IntToDouble` (`self.Demand`)) (`KismetMathLibrary.Conv_IntToDouble` (`self.iBaseNo`)))) -1))
    (switch `/Game/Blueprints/ERessorces` Ressoruce
      (:`NewEnumerator0`
        (set `self.Demand` 1))
      (:`NewEnumerator1`
        (set `self.Demand` 2))
      (:`NewEnumerator2`
        (set `self.Demand` 3)))
    (`/Game/Blueprints/LevelDatabseActor.AddDemand` _array_element (`self.iBaseNo`) (`self.Demand`))))

(fn `UserConstructionScript`)